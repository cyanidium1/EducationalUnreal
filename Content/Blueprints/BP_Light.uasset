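; BP_Light is a spotlight actor with an IsEnabled flag that sets the light's visibility in the Construction Script.
; Any actor overlap flips the flag at runtime, but the event graph never reapplies it to the SpotLight, so the toggle alone does not change the visible light.
; BeginPlay and overlap also print placeholder debug strings, and Tick is unused.
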(event EventBeginPlay
  (Development|PrintString "Hello"))

(event Collision|EventActorBeginOverlap
  (params (OtherActor :type Actor%20Object%20Reference))
  (Development|PrintString "kek")
  (if (Variables|Default|GetisEnabled)
    (Variables|Default|SetisEnabled false)
    (else
      (Variables|Default|SetisEnabled true))))

(event EventTick
  (params (DeltaSeconds :type Float%20%28single-precision%29)))

(fn ConstructionScript
  (Rendering|SetVisibility (Variables|Default|GetSpotLight) (Variables|Default|GetisEnabled) false))